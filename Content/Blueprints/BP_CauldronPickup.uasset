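; BP_CauldronPickup is a pickup Blueprint that plays a flame effect when collected.
; WasCollected attaches the P_Flamethrower emitter to PickupMesh, waits DelayTime, then calls the parent's WasCollected logic.
; Two unconnected addon snippets never run: one attaches the flame to the player's head socket, the other is an unfinished beam emitter toggle.
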(event `self.WasCollected`
  ;[1 1 1] Main
  (`GameplayStatics.SpawnEmitterAttached` "/Game/Realistic_Starter_VFX_Pack_Vol2/Particles/Fire/P_flamethrower.P_Flamethrower" (`self.PickupMesh`) "None" (0.0 0.0 0.0) (struct) (1.0 1.0 1.0) "SnapToTargetIncludingScale")
  (`KismetSystemLibrary.Delay` (`self.DelayTime`))
  (`parent.WasCollected`))

(fn `UserConstructionScript`)